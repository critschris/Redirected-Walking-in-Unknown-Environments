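; BP_MyXRPawn is an XR pawn with input for toggling a frozen camera view state.
; On BeginPlay it sets a local-floor tracking origin and adds the IMC_RDIE5 Enhanced Input mapping context.
; Holding IA_FreezeCamera sets FreezeView and stores the camera's world location and rotation, and completing or canceling it clears the flag.
; This graph only records that state and does not itself apply the frozen transform.
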(event Input|EnhancedActionEvents|EnhancedInputActionIA_FreezeCamera
  (params (ActionValue :type Boolean) (ElapsedSeconds :type Float%20%28double-precision%29) (TriggeredSeconds :type Float%20%28double-precision%29) (InputAction :type Input%20Action%20Object%20Reference :default "/Game/Input/IA_FreezeCamera.IA_FreezeCamera"))
  (bind _camera (Variables|Default|GetCamera))
  (:Started
    (Variables|Default|SetbFreezeView true)
    (Variables|Default|SetFrozenCameraLocation (Transformation|GetWorldLocation _camera))
    (Variables|Default|SetFrozenCameraRotation (Transformation|GetWorldRotation _camera)))
  (:Canceled
    (Variables|Default|SetbFreezeView false :!label _label))
  (:Completed
    (goto _label)))

(event EventBeginPlay
  (Class|HeadMountedDisplayFunctionLibrary|SetTrackingOrigin "LocalFloor")
  (Input|AddMappingContext (PlayerController|LocalPlayerSubsystems|GetEnhancedInputLocalPlayerSubsystem (Game|GetPlayerController 0)) "/Game/Input/IMC_RDIE5.IMC_RDIE5" 0 "(bIgnoreAllPressedKeysUntilRelease=True,bForceImmediately=False,bNotifyUserSettings=False)"))

(event Collision|EventActorBeginOverlap
  (params (OtherActor :type Actor%20Object%20Reference)))

(event EventTick
  (params (DeltaSeconds :type Float%20%28single-precision%29)))

(fn ConstructionScript)