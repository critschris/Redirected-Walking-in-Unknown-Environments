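; BP_WallFrontier is a wall boundary that computes a steering vector for a given player position, in the style of a potential field.
; The construction script sets the field's gain and falloff exponent and an initial State enum.
; CalculateSteeringVector scales the negated Frontier-to-player unit direction by Alpha and the gain, divided by distance raised to the exponent.
; The event graph is empty, so the vector is only computed when that function is called.
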(event EventBeginPlay)

(event Collision|EventActorBeginOverlap
  (params (OtherActor :type Actor%20Object%20Reference)))

(event EventTick
  (params (DeltaSeconds :type Float%20%28single-precision%29)))

(fn ConstructionScript
  (Variables|Default|Settheta_3 0.009)
  (Variables|Default|Settheta_4 2.5)
  (Variables|Default|SetState "NewEnumerator1"))

(fn CalculateSteeringVector
  (params (playerPos :type Vector))
  ;[0.15 0.15 0.15 0.5] ed_i
  (Variables|Default|Seted_i (Math|Vector|GetUnitDirection(Vector) (Transformation|GetWorldLocation (Variables|Default|GetFrontier)) playerPos))
  ;[0.15 0.15 0.15 0.5] d_i
  (Variables|Default|Setd_i (Math|Vector|Distance(Vector) playerPos (Transformation|GetWorldLocation (Variables|Default|GetFrontier))))
  (return (/ (* (Variables|Default|Getalpha) (* (Variables|Default|Gettheta_3) -1.0) (Variables|Default|Geted_i)) (Math|Float|Power (Math|Float|Absolute(Float) (Variables|Default|Getd_i)) (Variables|Default|Gettheta_4)))))