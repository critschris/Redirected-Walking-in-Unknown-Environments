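; FrontierManager is an actor that holds a list of frontier target points and computes a pull vector toward the current one from a given player position.
; ComputeCurrentTargetPointOutputVector negates the frontier-to-player direction, scales it by Alpha and Theta3, and divides by distance raised to Theta4, like a potential field.
; IncrementTargetPoint advances the index with no bounds check, and Tick prints that index for debugging.
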(event EventBeginPlay)

(event Collision|EventActorBeginOverlap
  (params (OtherActor :type Actor%20Object%20Reference)))

(event EventTick
  (params (DeltaSeconds :type Float%20%28single-precision%29))
  (Development|PrintString (Utilities|String|BuildString(Integer) "" "Current Index of Frontier array is: " (Variables|Default|Getindex)) true true "(R=0.000000,G=0.660000,B=1.000000,A=1.000000)" 2.0 "1"))

(fn ConstructionScript)

(fn ComputeCurrentTargetPointOutputVector
  (params (PlayerPOS :type Vector))
  (bind _frontiers (Variables|Default|GetFrontiers))
  (bind _index (Variables|Default|Getindex))
  (bind _output (Utilities|Array|Get(acopy) _frontiers _index))
  ;[0.15 0.15 0.15 0.5] ed_i
  (Variables|Default|Seted_i (Math|Vector|GetUnitDirection(Vector) _output PlayerPOS))
  ;[0.15 0.15 0.15 0.5] d_i
  (Variables|Default|Setd_i (Math|Vector|Distance(Vector) _output PlayerPOS))
  (return (/ (* (Variables|Default|Getalpha) (* (Variables|Default|Gettheta_3) -1.0) (Variables|Default|Geted_i)) (Math|Float|Power (Math|Float|Absolute(Float) (Variables|Default|Getd_i)) (Variables|Default|Gettheta_4)))))

(fn IncrementTargetPoint
  (Math|Integer|IncrementInt (Variables|Default|Getindex)))